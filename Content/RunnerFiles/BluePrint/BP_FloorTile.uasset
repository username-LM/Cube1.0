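; Floor tile for an endless runner that fills three lanes with random obstacles, bonus points, magnet and invisibility pickups on BeginPlay.
; Lanes chain middle, left, right with fresh rolls per check, so an empty result skips later lanes.
; It also spawns a Boost at the player once enough cubes are collected.
; When Boxyy overlaps EndTrigger, the game mode adds a tile and points, player speed rises within limits, and the tile destroys itself after a delay.
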(event OnComponentBeginOverlap(EndTrigger)
  (params (OverlappedComponent :type Primitive%20Component%20Object%20Reference) (OtherActor :type Actor%20Object%20Reference) (OtherComp :type Primitive%20Component%20Object%20Reference) (OtherBodyIndex :type Integer) (bFromSweep :type Boolean) (SweepResult :type Hit%20Result%20Structure%20%28by%20ref%29))
  (Utilities|Casting|CastToBoxyy OtherActor)
  (bind _asthird_person_game_mode (Utilities|Casting|CastToThirdPersonGameMode (Game|GetGameMode)))
  (Default|AddFloorTile _asthird_person_game_mode)
  (bind _asthird_person_game_mode_2 (Utilities|Casting|CastToThirdPersonGameMode (Game|GetGameMode)))
  (bind _output_get (Variables|/Game/ThirdPersonBP/Blueprints/ThirdPersonGameMode.ThirdPersonGameMode_C|SetCurrentPoints _asthird_person_game_mode_2 (+ (* 1 (Variables|/Game/ThirdPersonBP/Blueprints/ThirdPersonGameMode.ThirdPersonGameMode_C|GetPointsMultiplier _asthird_person_game_mode_2)) (Variables|/Game/ThirdPersonBP/Blueprints/ThirdPersonGameMode.ThirdPersonGameMode_C|GetCurrentPoints _asthird_person_game_mode_2))))
  (Development|PrintString (Utilities|String|ToString(Integer) _output_get))
  (bind _asboxyy (Utilities|Casting|CastToBoxyy (Game|GetPlayerCharacter 0)))
  (Variables|/Script/Engine.CharacterMovementComponent|SetMaxWalkSpeed (Variables|/Script/Engine.Character|GetCharacterMovement _asboxyy) (Math|Float|Clamp(Float) (* (Variables|/Script/Engine.CharacterMovementComponent|GetMaxWalkSpeed (Variables|/Script/Engine.Character|GetCharacterMovement _asboxyy)) 1.008) 1e+03 4.5e+03))
  (Utilities|FlowControl|Delay 2.0)
  (Actor|DestroyActor))

(event EventBeginPlay
  (CallFunction|SpawnObstacles))

(event Collision|EventActorBeginOverlap
  (params (OtherActor :type Actor%20Object%20Reference)))

(event EventTick
  (params (DeltaSeconds :type Float%20%28single-precision%29)))

(fn ConstructionScript)

(fn SpawnPoint
  (return (Transformation|GetWorldTransform (Variables|Default|GetAttachPoint))))

(fn SpawnObstacles
  (bind _returnvalue (Math|Random|RandomFloatinRange 0.0 1.0))
  (bind _returnvalue_2 (Math|Random|RandomFloatinRange 0.0 1.0))
  (bind _returnvalue_3 (Math|Random|RandomFloatinRange 0.0 1.0))
  (bind _arrow1 (Variables|Default|GetArrow1))
  (bind _arrow0 (Variables|Default|GetArrow0))
  (bind _arrow2 (Variables|Default|GetArrow2))
  (bind _returnvalue_4 (Transformation|GetWorldTransform _arrow1))
  (bind _returnvalue_5 (Transformation|GetWorldTransform _arrow0))
  (bind _returnvalue_6 (Transformation|GetWorldTransform _arrow2))
  (bind _asthird_person_game_mode (Utilities|Casting|CastToThirdPersonGameMode (Game|GetGameMode)))
  (bind _asboxyy (Utilities|Casting|CastToBoxyy (Game|GetPlayerCharacter 0)))
  (Utilities|FlowControl|Sequence
    (:then_0
      ;[1 1 1] LANE2(MIDDLE)
      (if (Math|Float|InRange(Float) _returnvalue 0.0 0.3)
        (Game|SpawnActorfromClass "/Game/RunnerFiles/BluePrint/ObstacleLow.ObstacleLow_C" _returnvalue_4 "Undefined" 0 0)
        ;[1 1 1] LANE1_LEFT
        (if (Math|Float|InRange(Float) _returnvalue_2 0.0 0.4) :!label _label
          (Game|SpawnActorfromClass "/Game/RunnerFiles/BluePrint/ObstacleLow.ObstacleLow_C" _returnvalue_5 "Undefined" 0 0)
          ;[1 1 1] LANE3_RIGHT
          (if (Math|Float|InRange(Float) _returnvalue_3 0.0 0.4) :!label _label_2
            (Game|SpawnActorfromClass "/Game/RunnerFiles/BluePrint/ObstacleLow.ObstacleLow_C" _returnvalue_6 "Undefined" 0 0)
            (elif (Math|Float|InRange(Float) _returnvalue_3 0.4 0.5)
              (Game|SpawnActorfromClass "/Game/RunnerFiles/BluePrint/ObstacleHigh.ObstacleHigh_C" _returnvalue_6 "Undefined" 0 0)
              (elif (Math|Float|InRange(Float) _returnvalue_3 0.5 0.85)
                (Game|SpawnActorfromClass "/Game/RunnerFiles/BluePrint/BonusPoints.BonusPoints_C" _returnvalue_6 "Undefined" 0 0)
                (elif (and (Math|Float|InRange(Float) _returnvalue_3 0.85 0.95) (not (Variables|/Game/ThirdPersonBP/Blueprints/Boxyy.Boxyy_C|GetMagnetActive _asboxyy)))
                  (Game|SpawnActorfromClass "/Game/RunnerFiles/magnet_jump/magnet2.magnet2_C" _returnvalue_6 "Undefined" 0 0)
                  (elif (and (Math|Float|InRange(Float) _returnvalue_3 0.95 1.0) (not (Variables|/Game/ThirdPersonBP/Blueprints/Boxyy.Boxyy_C|GetInvisibilityActive _asboxyy)))
                    (Game|SpawnActorfromClass "/Game/RunnerFiles/magnet_jump/Invisibility2.Invisibility2_C" _returnvalue_6 "Undefined" 0 0))))))
          (elif (Math|Float|InRange(Float) _returnvalue_2 0.4 0.5)
            (Game|SpawnActorfromClass "/Game/RunnerFiles/BluePrint/ObstacleHigh.ObstacleHigh_C" _returnvalue_5 "Undefined" 0 0)
            (goto _label_2)
            (elif (Math|Float|InRange(Float) _returnvalue_2 0.5 0.85)
              (Game|SpawnActorfromClass "/Game/RunnerFiles/BluePrint/BonusPoints.BonusPoints_C" _returnvalue_5 "Undefined" 0 0)
              (goto _label_2)
              (elif (and (Math|Float|InRange(Float) _returnvalue_2 0.85 0.95) (not (Variables|/Game/ThirdPersonBP/Blueprints/Boxyy.Boxyy_C|GetMagnetActive _asboxyy)))
                (Game|SpawnActorfromClass "/Game/RunnerFiles/magnet_jump/magnet2.magnet2_C" _returnvalue_5 "Undefined" 0 0)
                (goto _label_2)
                (elif (and (Math|Float|InRange(Float) _returnvalue_2 0.95 1.0) (not (Variables|/Game/ThirdPersonBP/Blueprints/Boxyy.Boxyy_C|GetInvisibilityActive _asboxyy)))
                  (Game|SpawnActorfromClass "/Game/RunnerFiles/magnet_jump/Invisibility2.Invisibility2_C" _returnvalue_5 "Undefined" 0 0)
                  (goto _label_2))))))
        (elif (Math|Float|InRange(Float) _returnvalue 0.3 0.5)
          (Game|SpawnActorfromClass "/Game/RunnerFiles/BluePrint/ObstacleHigh.ObstacleHigh_C" _returnvalue_4 "Undefined" 0 0)
          (goto _label)
          (elif (Math|Float|InRange(Float) _returnvalue 0.5 0.8)
            (Game|SpawnActorfromClass "/Game/RunnerFiles/BluePrint/BonusPoints.BonusPoints_C" _returnvalue_4 "Undefined" 0 0)
            (goto _label)
            (elif (and (Math|Float|InRange(Float) _returnvalue 0.85 0.95) (not (Variables|/Game/ThirdPersonBP/Blueprints/Boxyy.Boxyy_C|GetMagnetActive _asboxyy)))
              (Game|SpawnActorfromClass "/Game/RunnerFiles/magnet_jump/magnet2.magnet2_C" _returnvalue_4 "Undefined" 0 0)
              (goto _label)
              (elif (and (Math|Float|InRange(Float) _returnvalue 0.95 1.0) (not (Variables|/Game/ThirdPersonBP/Blueprints/Boxyy.Boxyy_C|GetInvisibilityActive _asboxyy)))
                (Game|SpawnActorfromClass "/Game/RunnerFiles/magnet_jump/Invisibility2.Invisibility2_C" _returnvalue_4 "Undefined" 0 0)
                (goto _label)))))))
    (:then_1
      (if (and (not (Variables|/Game/ThirdPersonBP/Blueprints/Boxyy.Boxyy_C|GetBonusActive _asboxyy)) (>= (Variables|/Game/ThirdPersonBP/Blueprints/ThirdPersonGameMode.ThirdPersonGameMode_C|GetCurrentCubesValue _asthird_person_game_mode) 30))
        (if (not (Variables|Default|GetBoostSpawned))
          (Utilities|FlowControl|Sequence
            (:then_0
              (Game|SpawnActorfromClass "/Game/RunnerFiles/magnet_jump/Boost.Boost_C" (Math|Conversions|ToTransform(Vector) (+ (Math|Vector|MakeVector (.x (Transformation|GetWorldLocation (Variables|/Script/Engine.Character|GetCapsuleComponent _asboxyy))) (.y (Transformation|GetWorldLocation (Variables|/Script/Engine.Character|GetCapsuleComponent _asboxyy))) (.z (Transformation|GetWorldLocation (Variables|/Script/Engine.Character|GetCapsuleComponent _asboxyy)))) 0)) "Undefined" 0 0))
            (:then_1
              (Variables|Default|SetBoostSpawned true))))))))